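; NPC actor that turns its mesh toward the player and shows dialogue when something enters its trigger.
; Every Tick it yaws the mesh toward the first-person camera, ignoring height, with pitch fixed at -90.
; The first overlap creates a WG_Dialogue widget, later ones unhide it, and each calls Lancement with QuelleDialoque.
; Leaving hides the widget and passes the first enum value; neither overlap event filters the actor.
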(event OnComponentBeginOverlap(TriggerDialogue)
  (params (OverlappedComponent :type Primitive%20Component%20Object%20Reference) (OtherActor :type Actor%20Object%20Reference) (OtherComp :type Primitive%20Component%20Object%20Reference) (OtherBodyIndex :type Integer) (bFromSweep :type Boolean) (SweepResult :type Hit%20Result%20Structure%20%28by%20ref%29))
  (if (Variables|Default|Getpremiere%20fois)
    (Variables|Default|Setpremiere%20fois false)
    (bind _returnvalue (UserInterface|CreateWidget "/Game/Widget/Dialogue/WG_Dialogue.WG_Dialogue_C"))
    (bind _output_get (Variables|Default|SetRefWidget _returnvalue))
    (UserInterface|Viewport|AddtoViewport _output_get 0)
    (else
      (Widget|SetVisibility (Variables|Default|GetRefWidget) "Visible")))
  (Default|Lancement _output_get (Variables|Default|GetQuelleDialoque)))

(event OnComponentEndOverlap(TriggerDialogue)
  (params (OverlappedComponent :type Primitive%20Component%20Object%20Reference) (OtherActor :type Actor%20Object%20Reference) (OtherComp :type Primitive%20Component%20Object%20Reference) (OtherBodyIndex :type Integer))
  (bind _refwidget (Variables|Default|GetRefWidget))
  (Widget|SetVisibility _refwidget "Hidden")
  (Default|Lancement _refwidget "NewEnumerator0"))

(event EventBeginPlay)

(event Collision|EventActorBeginOverlap
  (params (OtherActor :type Actor%20Object%20Reference)))

(event EventTick
  (params (DeltaSeconds :type Float%20%28single-precision%29))
  (bind _returnvalue (Game|GetPlayerCharacter 0))
  (bind _npc_mesh (Variables|Default|GetNPC_Mesh))
  (bind _returnvalue_2 (Transformation|GetWorldLocation _npc_mesh))
  (bind _asbp_first_person_character (Utilities|Casting|CastToBP_FirstPersonCharacter _returnvalue))
  (bind _firstpersoncamera (Variables|/Game/FirstPerson/Blueprints/BP_FirstPersonCharacter.BP_FirstPersonCharacter_C|GetFirstPersonCamera _asbp_first_person_character))
  (bind _returnvalue_3 (Transformation|GetWorldLocation _firstpersoncamera))
  (bind _returnvalue_4 (Math|Rotator|FindLookatRotation (Math|Vector|MakeVector (.x _returnvalue_2) (.y _returnvalue_2) 0.0) (Math|Vector|MakeVector (.x _returnvalue_3) (.y _returnvalue_3) 0.0)))
  (Transformation|SetWorldRotation (Variables|Default|GetNPC_Mesh) (Math|Rotator|MakeRotator (.roll _returnvalue_4) -9e+01 (.yaw _returnvalue_4)) false false))

(fn ConstructionScript)
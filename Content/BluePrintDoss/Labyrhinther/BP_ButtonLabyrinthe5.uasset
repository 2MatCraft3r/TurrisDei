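; Labyrinth button Blueprint for the fifth crystal, which the player can activate once to drive the "Rune5" parameter.
; A box overlap shows a prompt plane that turns toward the player's camera every Tick, until the crystal is activated.
; Interaction plays a sound, changes the ball's material, turns off the light and notifies verification and counter logic.
; A timeline then animates the rune in the Scal_Porte material parameter collection.
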(event OnComponentBeginOverlap(Box)
  (params (OverlappedComponent :type Primitive%20Component%20Object%20Reference) (OtherActor :type Actor%20Object%20Reference) (OtherComp :type Primitive%20Component%20Object%20Reference) (OtherBodyIndex :type Integer) (bFromSweep :type Boolean) (SweepResult :type Hit%20Result%20Structure%20%28by%20ref%29))
  (if (not (Variables|Default|GetActiver5))
    (if (== OtherActor (Variables|Default|GetRefplayer))
      (Rendering|SetVisibility (Variables|Default|GetPlane) true false))))

(event OnComponentEndOverlap(Box)
  (params (OverlappedComponent :type Primitive%20Component%20Object%20Reference) (OtherActor :type Actor%20Object%20Reference) (OtherComp :type Primitive%20Component%20Object%20Reference) (OtherBodyIndex :type Integer))
  (if (== (Variables|Default|GetRefplayer) OtherActor)
    (Rendering|SetVisibility (Variables|Default|GetPlane) false false)))

(event EventBeginPlay
  (bind _asbp_first_person_character (Utilities|Casting|CastToBP_FirstPersonCharacter (Game|GetPlayerCharacter 0)))
  (Variables|Default|SetRefPLayer _asbp_first_person_character))

(event Collision|EventActorBeginOverlap
  (params (OtherActor :type Actor%20Object%20Reference)))

(event EventTick
  (params (DeltaSeconds :type Float%20%28single-precision%29))
  (bind _plane (Variables|Default|GetPlane))
  (bind _refplayer (Variables|Default|GetRefplayer))
  (bind _returnvalue (Transformation|GetWorldLocation _plane))
  (bind _firstpersoncamera (Variables|/Game/FirstPerson/Blueprints/BP_FirstPersonCharacter.BP_FirstPersonCharacter_C|GetFirstPersonCamera _refplayer))
  (bind _returnvalue_2 (Transformation|GetWorldLocation _firstpersoncamera))
  (bind _returnvalue_3 (Math|Rotator|FindLookatRotation _returnvalue _returnvalue_2))
  (Transformation|SetWorldRotation (Variables|Default|GetPlane) (Math|Rotator|MakeRotator (+ (.roll _returnvalue_3) 9e+01) 0.0 (+ (.yaw _returnvalue_3) -9e+01)) false false))

(event EventInteraction
  (if (not (Variables|Default|GetActiver5))
    (Audio|PlaySound2D "/Game/Sound/BPSound/crystal_activated.crystal_activated" 0.5 1.0 0.5 0 0)
    (Variables|Default|SetActiver5 true)
    (Rendering|Material|SetMaterial (Variables|Default|GetCristaleBall) 0 0)
    (Default|Verification (Variables|Default|GetRefVerif))
    (Default|Compteur (Variables|/Game/FirstPerson/Blueprints/BP_FirstPersonCharacter.BP_FirstPersonCharacter_C|GetrefButton (Variables|Default|GetRefplayer)))
    (Rendering|Components|Light|SetIntensity (Variables|Default|GetPointLight) 0.0)
    (bind _newtrack_0 (Timeline|Timeline Play)
      (:Update
        (Rendering|Material|SetScalarParameterValue "/Game/Asset/Texture/TEX_Porte/Scal_Porte.Scal_Porte" "Rune5" _newtrack_0 :!class /Script/Engine.KismetMaterialLibrary)
        (Rendering|SetVisibility (Variables|Default|GetPlane) false false)))))

(fn ConstructionScript
  (Rendering|Components|Light|SetIntensity (Variables|Default|GetPointLight) (Variables|Default|GetNew%20Intensity)))
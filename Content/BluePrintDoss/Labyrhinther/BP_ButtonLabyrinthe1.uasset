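; BP_ButtonLabyrinthe1 is a one-shot interactable labyrinth button, apparently the first of several, that lights a rune.
; On Interaction it latches Activer1, swaps the sphere's material, switches off its point light, and calls Verification on RefVerif and Compteur on the player's RefButton.
; A timeline then animates the Rune1 scalar in the Scal_Porte Material Parameter Collection.
; The construction script sets the light's starting intensity.
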(event EventBeginPlay
  (bind _asbp_first_person_character (Utilities|Casting|CastToBP_FirstPersonCharacter (Game|GetPlayerCharacter 0)))
  (Variables|Default|SetRefplayer _asbp_first_person_character))

(event Collision|EventActorBeginOverlap
  (params (OtherActor :type Actor%20Object%20Reference)))

(event EventTick
  (params (DeltaSeconds :type Float%20%28single-precision%29)))

(event EventInteraction
  (if (not (Variables|Default|GetActiver1))
    (Variables|Default|SetActiver1 true)
    (Rendering|Material|SetMaterial (Variables|Default|GetSphere) 0 0)
    (Default|Verification (Variables|Default|GetRefVerif))
    (Default|Compteur (Variables|/Game/FirstPerson/Blueprints/BP_FirstPersonCharacter.BP_FirstPersonCharacter_C|GetrefButton (Variables|Default|GetRefplayer)))
    (Rendering|Components|Light|SetIntensity (Variables|Default|GetPointLight) 0.0)
    (bind _newtrack_0 (Timeline|Timeline Play)
      (:Update
        (Rendering|Material|SetScalarParameterValue "/Game/Asset/Texture/TEX_Porte/Scal_Porte.Scal_Porte" "Rune1" _newtrack_0 :!class /Script/Engine.KismetMaterialLibrary)))))

(fn ConstructionScript
  (Rendering|Components|Light|SetIntensity (Variables|Default|GetPointLight) (Variables|Default|GetNew%20Intensity)))
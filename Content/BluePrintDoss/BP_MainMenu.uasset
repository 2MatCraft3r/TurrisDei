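; BP_MainMenu is an actor that serves as the main menu's camera view.
; On BeginPlay it makes itself the player's view target, shows the mouse cursor and sets CanBubbleHead to false on the BP_FirstPersonCharacter.
; A Zoom event plays a timeline that lerps its camera's field of view from wide to narrow.
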(event Custom|Zoom
  (bind _newtrack_0 (Timeline|Timeline Play)
    (:Update
      (Camera|SetFieldOfView (Variables|Default|GetCamera) (Math|Float|Lerp 9e+01 5e+01 _newtrack_0)))))

(event EventBeginPlay
  (bind _returnvalue (Game|GetPlayerController 0))
  (Variables|/Game/FirstPerson/Blueprints/BP_FirstPersonCharacter.BP_FirstPersonCharacter_C|SetCanBubleHead (.AsBP%20First%20Person%20Character (Utilities|Casting|CastToBP_FirstPersonCharacter (Game|GetPlayerCharacter 0))) false)
  (Game|Player|SetViewTargetwithBlend _returnvalue self 0.0 "VTBlend_Linear" 0.0 false)
  (Variables|/Script/Engine.PlayerController|SetbShowMouseCursor _returnvalue true))

(event Collision|EventActorBeginOverlap
  (params (OtherActor :type Actor%20Object%20Reference)))

(event EventTick
  (params (DeltaSeconds :type Float%20%28single-precision%29)))

(fn ConstructionScript)
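; Fireplace trap actor that plays a positional fire sound near the player and vanishes in a light flash when its box is overlapped.
; DetectionSon overlaps toggle an in-range flag, which Tick reads through DoOnce gates to spawn the sound on first entry, then stop or replay it.
; Any Box overlap briefly flares the light, hides three plane actors, stops the sound and destroys the actor.
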(event OnComponentBeginOverlap(Box)
  (params (OverlappedComponent :type Primitive%20Component%20Object%20Reference) (OtherActor :type Actor%20Object%20Reference) (OtherComp :type Primitive%20Component%20Object%20Reference) (OtherBodyIndex :type Integer) (bFromSweep :type Boolean) (SweepResult :type Hit%20Result%20Structure%20%28by%20ref%29))
  (bind _light (Variables|Default|GetLight))
  (bind _lightcomponent (Variables|/Script/Engine.Light|GetLightComponent _light))
  (Rendering|Components|Light|SetIntensity _lightcomponent 1e+04)
  (Utilities|FlowControl|Delay 0.4)
  (Rendering|Components|Light|SetIntensity _lightcomponent 0.0)
  (Rendering|SetActorHiddenInGame (Variables|Default|GetPlane) true)
  (Audio|Components|Audio|Stop (Variables|Default|GetWhisperr))
  (Actor|DestroyActor))

(event OnComponentBeginOverlap(DetectionSon)
  (params (OverlappedComponent :type Primitive%20Component%20Object%20Reference) (OtherActor :type Actor%20Object%20Reference) (OtherComp :type Primitive%20Component%20Object%20Reference) (OtherBodyIndex :type Integer) (bFromSweep :type Boolean) (SweepResult :type Hit%20Result%20Structure%20%28by%20ref%29))
  ;[1 1 1] Porte
  (Utilities|Casting|CastToBP_FirstPersonCharacter (Game|GetPlayerCharacter 0))
  (Variables|Default|SetAporter true))

(event OnComponentEndOverlap(DetectionSon)
  (params (OverlappedComponent :type Primitive%20Component%20Object%20Reference) (OtherActor :type Actor%20Object%20Reference) (OtherComp :type Primitive%20Component%20Object%20Reference) (OtherBodyIndex :type Integer))
  ;[1 1 1] Porte
  (Utilities|Casting|CastToBP_FirstPersonCharacter (Game|GetPlayerCharacter 0))
  (Variables|Default|SetAporter false))

(event EventBeginPlay)

(event Collision|EventActorBeginOverlap
  (params (OtherActor :type Actor%20Object%20Reference)))

(event EventTick
  (params (DeltaSeconds :type Float%20%28single-precision%29))
  ;[1 1 1] GestyionSon
  (if (Variables|Default|GetAporter)
    (Utilities|FlowControl|Sequence
      (:then_0
        (if (Variables|Default|GetFirstTime)
          (Variables|Default|SetFirstTime false)
          (Utilities|FlowControl|DoOnce false
            (:Completed
              (Development|PrintString "play")
              (bind _returnvalue (Audio|SpawnSoundatLocation "/Game/StarterContent/Audio/Fire01.Fire01" (Transformation|GetWorldLocation (Variables|Default|GetDetectionSon)) "0, 0, 0" 0.2 1.0 0.0 "/Game/Sound/BPSound/ATT_Piege.ATT_Piege" 0 false))
              (Variables|Default|SetWhisperr _returnvalue)))
          (else
            (Utilities|FlowControl|DoOnce false :!label _label
              (:Completed
                (Audio|Components|Audio|Play (Variables|Default|GetWhisperr) 0.0))))))
      (:then_1
        (goto _label_2 Reset)))
    (else
      (Utilities|FlowControl|Sequence
        (:then_0
          (Utilities|FlowControl|DoOnce true :!label _label_2
            (:Completed
              (Audio|Components|Audio|Stop (Variables|Default|GetWhisperr)))))
        (:then_1
          (goto _label Reset))))))

(fn ConstructionScript)
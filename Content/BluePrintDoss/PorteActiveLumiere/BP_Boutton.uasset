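; Light-activated button that opens its referenced door when the player stays in its detection zone with their light active.
; It re-checks on zone entry and on the player character's Sort2Valid event, then runs a timeline as a charge timer.
; The sphere switches to the sun-on material partway through, and reverts if the player leaves or the light goes off, stopping the timeline.
; On completion it calls Ouverture on the door and destroys itself.
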(event OnComponentBeginOverlap(ZoneDedetection)
  (params (OverlappedComponent :type Primitive%20Component%20Object%20Reference) (OtherActor :type Actor%20Object%20Reference) (OtherComp :type Primitive%20Component%20Object%20Reference) (OtherBodyIndex :type Integer) (bFromSweep :type Boolean) (SweepResult :type Hit%20Result%20Structure%20%28by%20ref%29))
  (if (== OtherActor (.AsBP%20First%20Person%20Character (Utilities|Casting|CastToBP_FirstPersonCharacter (Game|GetPlayerCharacter 0))))
    (Variables|Default|SetDansLaZone true)
    (if (and (Variables|Default|GetDansLaZone) (Variables|/Game/FirstPerson/Blueprints/BP_FirstPersonCharacter.BP_FirstPersonCharacter_C|GetLumiereActive (.AsBP%20First%20Person%20Character (Utilities|Casting|CastToBP_FirstPersonCharacter (Game|GetPlayerCharacter 0)))))
      (bind _newtrack_0 (Timeline|Timeline PlayFromStart)
        (:Update
          (if (and (Variables|Default|GetDansLaZone) (Variables|/Game/FirstPerson/Blueprints/BP_FirstPersonCharacter.BP_FirstPersonCharacter_C|GetLumiereActive (.AsBP%20First%20Person%20Character (Utilities|Casting|CastToBP_FirstPersonCharacter (Game|GetPlayerCharacter 0)))))
            (Variables|Default|SetCurentTime _newtrack_0)
            (if (> (Variables|Default|GetCurentTime) 1.5)
              (Rendering|Material|SetMaterial (Variables|Default|GetSphere) 0 "/Game/VFX/M_SunOn.M_SunOn"))
            (else
              (Rendering|Material|SetMaterial (Variables|Default|GetSphere) 0 "/Game/VFX/M_SunOff.M_SunOff")
              (Timeline|Timeline Stop))))
        (:Finished
          (Default|Ouverture (Variables|Default|GetPorteRef))
          (Actor|DestroyActor))))))

(event OnComponentEndOverlap(ZoneDedetection)
  (params (OverlappedComponent :type Primitive%20Component%20Object%20Reference) (OtherActor :type Actor%20Object%20Reference) (OtherComp :type Primitive%20Component%20Object%20Reference) (OtherBodyIndex :type Integer))
  (Variables|Default|SetDansLaZone false))

(event Custom|Activelumm
  (if (and (Variables|Default|GetDansLaZone) (Variables|/Game/FirstPerson/Blueprints/BP_FirstPersonCharacter.BP_FirstPersonCharacter_C|GetLumiereActive (.AsBP%20First%20Person%20Character (Utilities|Casting|CastToBP_FirstPersonCharacter (Game|GetPlayerCharacter 0)))))
    (bind _newtrack_0 (Timeline|Timeline PlayFromStart)
      (:Update
        (if (and (Variables|Default|GetDansLaZone) (Variables|/Game/FirstPerson/Blueprints/BP_FirstPersonCharacter.BP_FirstPersonCharacter_C|GetLumiereActive (.AsBP%20First%20Person%20Character (Utilities|Casting|CastToBP_FirstPersonCharacter (Game|GetPlayerCharacter 0)))))
          (Variables|Default|SetCurentTime _newtrack_0)
          (if (> (Variables|Default|GetCurentTime) 1.5)
            (Rendering|Material|SetMaterial (Variables|Default|GetSphere) 0 "/Game/VFX/M_SunOn.M_SunOn"))
          (else
            (Rendering|Material|SetMaterial (Variables|Default|GetSphere) 0 "/Game/VFX/M_SunOff.M_SunOff")
            (Timeline|Timeline Stop))))
      (:Finished
        (Default|Ouverture (Variables|Default|GetPorteRef))
        (Actor|DestroyActor)))))

(event EventBeginPlay
  (bind _asbp_first_person_character (Utilities|Casting|CastToBP_FirstPersonCharacter (Game|GetPlayerCharacter 0)))
  (EventDispatchers|BindEventtoSort2Valid _asbp_first_person_character (delegate Custom|Activelumm)))

(event Collision|EventActorBeginOverlap
  (params (OtherActor :type Actor%20Object%20Reference)))

(event EventTick
  (params (DeltaSeconds :type Float%20%28single-precision%29)))

(fn ConstructionScript)
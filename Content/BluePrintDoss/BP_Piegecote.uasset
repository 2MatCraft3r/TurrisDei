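; BP_Piegecote is a side trap with a platform that slides back and forth and a death volume that sends the player back to respawn.
; From BeginPlay, a Timeline lerps the platform's relative Y between start and travel distances, with a FlipFlop reversing or replaying it after a short pause.
; Any overlap with Mort moves the first-person character's capsule to its stored ReSpawn transform, without checking what overlapped.
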(event OnComponentBeginOverlap(Mort)
  (params (OverlappedComponent :type Primitive%20Component%20Object%20Reference) (OtherActor :type Actor%20Object%20Reference) (OtherComp :type Primitive%20Component%20Object%20Reference) (OtherBodyIndex :type Integer) (bFromSweep :type Boolean) (SweepResult :type Hit%20Result%20Structure%20%28by%20ref%29))
  (bind _returnvalue (Game|GetPlayerCharacter 0))
  (bind _asbp_first_person_character (Utilities|Casting|CastToBP_FirstPersonCharacter _returnvalue))
  (Transformation|SetWorldTransform (Variables|/Script/Engine.Character|GetCapsuleComponent _asbp_first_person_character) (Variables|/Game/FirstPerson/Blueprints/BP_FirstPersonCharacter.BP_FirstPersonCharacter_C|GetReSpawn _asbp_first_person_character) false false))

(event Custom|Deplacement
  (bind _newtrack_0 (Timeline|Timeline Play)
    (:Update
      (Transformation|SetRelativeLocation (Variables|Default|GetPlatform) (Math|Vector|MakeVector 0.0 (Math|Float|Lerp (Variables|Default|GetDistanceDepart) (Variables|Default|GetDistanceDeplacement) _newtrack_0) 0.0) false false))
    (:Finished
      (Utilities|FlowControl|FlipFlop
        (:A
          (Utilities|FlowControl|Delay 0.2)
          (Timeline|Timeline Reverse))
        (:B
          (Utilities|FlowControl|Delay 0.8)
          (Timeline|Timeline PlayFromStart))))))

(event EventBeginPlay
  (CallFunction|Deplacement))

(event Collision|EventActorBeginOverlap
  (params (OtherActor :type Actor%20Object%20Reference)))

(event EventTick
  (params (DeltaSeconds :type Float%20%28single-precision%29)))

(fn ConstructionScript)
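; BP_ToucheInfo is a trigger actor that shows a WG_Touche widget, apparently a key hint, while the first-person player is inside its Box.
; On first entry it creates the widget and adds it to the viewport; later entries reuse and unhide it.
; Each entry passes QuelleTouche ("which key") to the widget's Lancementt function, and leaving the box hides the widget.
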(event OnComponentBeginOverlap(Box)
  (params (OverlappedComponent :type Primitive%20Component%20Object%20Reference) (OtherActor :type Actor%20Object%20Reference) (OtherComp :type Primitive%20Component%20Object%20Reference) (OtherBodyIndex :type Integer) (bFromSweep :type Boolean) (SweepResult :type Hit%20Result%20Structure%20%28by%20ref%29))
  (if (== OtherActor (Variables|Default|GetPlayerRef))
    (if (Variables|Default|GetPremiereFois)
      (Variables|Default|SetPremiereFois false)
      (bind _returnvalue (UserInterface|CreateWidget "/Game/Widget/Dialogue/WG_Touche.WG_Touche_C"))
      (bind _output_get (Variables|Default|SetRefWidget _returnvalue))
      (UserInterface|Viewport|AddtoViewport _output_get 0)
      (else
        (Widget|SetVisibility (Variables|Default|GetRefWidget) "Visible")))
    (Default|Lancementt _output_get (Variables|Default|GetQuelleTouche))))

(event OnComponentEndOverlap(Box)
  (params (OverlappedComponent :type Primitive%20Component%20Object%20Reference) (OtherActor :type Actor%20Object%20Reference) (OtherComp :type Primitive%20Component%20Object%20Reference) (OtherBodyIndex :type Integer))
  (if (== OtherActor (Variables|Default|GetPlayerRef))
    (Widget|SetVisibility (Variables|Default|GetRefWidget) "Hidden")))

(event EventBeginPlay
  (bind _asbp_first_person_character (Utilities|Casting|CastToBP_FirstPersonCharacter (Game|GetPlayerCharacter 0)))
  (Variables|Default|SetPlayerRef _asbp_first_person_character))

(event Collision|EventActorBeginOverlap
  (params (OtherActor :type Actor%20Object%20Reference)))

(event EventTick
  (params (DeltaSeconds :type Float%20%28single-precision%29)))

(fn ConstructionScript)
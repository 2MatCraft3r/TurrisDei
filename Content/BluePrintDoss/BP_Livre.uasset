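; BP_Livre is the interactable book that gives the player the magic book and triggers a cinematic leading into the tutorial.
; It starts hidden with Donatien; interaction enables the player's book and magic VFX, turns off its light and clears an environment mesh.
; It then reveals a portal and plays Donatien's montage with timed Niagara effects and a notify-driven screen fade.
; On completion it destroys both actors and passes the monster spawn and movement zone to the player's ScriptTuto.
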(event EventBeginPlay
  (Rendering|SetActorHiddenInGame (Variables|Default|GetDonatien) true)
  (bind _asbp_first_person_character (Utilities|Casting|CastToBP_FirstPersonCharacter (Game|GetPlayerCharacter 0)))
  (Variables|Default|SetRefPlayer _asbp_first_person_character)
  (Rendering|SetActorHiddenInGame true))

(event Collision|EventActorBeginOverlap
  (params (OtherActor :type Actor%20Object%20Reference)))

(event EventTick
  (params (DeltaSeconds :type Float%20%28single-precision%29)))

(event EventInteraction
  (bind _returnvalue (Game|GetPlayerCharacter 0))
  (bind _donatien (Variables|Default|GetDonatien))
  (bind _refplayer (Variables|Default|GetRefPlayer))
  (bind _asbp_first_person_character (Utilities|Casting|CastToBP_FirstPersonCharacter _returnvalue))
  (bind _reftransi (Variables|/Game/FirstPerson/Blueprints/BP_FirstPersonCharacter.BP_FirstPersonCharacter_C|GetRefTransi _refplayer))
  (Utilities|FlowControl|Sequence
    (:then_0
      (Components|Activation|SetActive (Variables|/Game/FirstPerson/Blueprints/BP_FirstPersonCharacter.BP_FirstPersonCharacter_C|GetVFXMagie _asbp_first_person_character) true false)
      (Variables|/Game/FirstPerson/Blueprints/BP_FirstPersonCharacter.BP_FirstPersonCharacter_C|SetCanLivre _asbp_first_person_character true)
      (Rendering|SetVisibility (Variables|/Game/FirstPerson/Blueprints/BP_FirstPersonCharacter.BP_FirstPersonCharacter_C|GetLivre _asbp_first_person_character) true false)
      (Rendering|Components|Light|SetIntensity (Variables|/Game/FirstPerson/Blueprints/BP_FirstPersonCharacter.BP_FirstPersonCharacter_C|GetLivreLight _asbp_first_person_character) 0.0)
      (Variables|/Game/FirstPerson/Blueprints/BP_FirstPersonCharacter.BP_FirstPersonCharacter_C|SetLumiereActive _asbp_first_person_character false)
      (Components|StaticMesh|SetStaticMesh (Variables|Default|GetENV_Livre_pCube15) 0))
    (:then_1
      (Development|SetHiddeninGame (Variables|/Game/Animations/Donatien/VFX_Portal.VFX_Portal_C|GetPortalAnim (Variables|Default|GetPortal)) false false)
      (Utilities|FlowControl|Delay 1.0)
      (Rendering|SetActorHiddenInGame _donatien false)
      (Animation|Montage|PlayMontage (Variables|/Script/Engine.SkeletalMeshActor|GetSkeletalMeshComponent _donatien) "/Game/Animations/Donatien/Donatien_Cinematique_Montage.Donatien_Cinematique_Montage"
        (:then
          (Utilities|FlowControl|Delay 1.5)
          (Components|Activation|SetActive (Variables|Default|GetNiagara) true false)
          (Utilities|FlowControl|Delay 5.0)
          (Components|DestroyComponent (Variables|Default|GetNiagara)))
        (:OnCompleted
          (Actor|DestroyActor (Variables|Default|GetDonatien))
          (Default|ScriptTuto (Variables|Default|GetRefPlayer) (Variables|Default|GetSpawnMonstre) (Variables|Default|GetZoneDeplacement)))
        (:OnNotifyBegin
          (Widget|SetVisibility _reftransi "Visible")
          (Default|FadeMorte _reftransi)
          (Utilities|FlowControl|Delay 2.5)
          (Default|FadeEnd _reftransi)
          (Utilities|FlowControl|Delay 0.8)
          (Widget|SetVisibility _reftransi "Hidden"))))))

(fn ConstructionScript)
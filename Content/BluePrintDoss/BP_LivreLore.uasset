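; BP_LivreLore is a lore book actor that opens a text screen when interacted with.
; A Box overlap sets the InBox flag and toggles the InteractIcon as an in-range prompt.
; The Interaction event creates a WG_TexteLore widget from the book's IDTexte and adds it to the viewport.
; It then disables move, look, power and interact on the cached first-person character, with no re-enable in this Blueprint.
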(event OnComponentBeginOverlap(Box)
  (params (OverlappedComponent :type Primitive%20Component%20Object%20Reference) (OtherActor :type Actor%20Object%20Reference) (OtherComp :type Primitive%20Component%20Object%20Reference) (OtherBodyIndex :type Integer) (bFromSweep :type Boolean) (SweepResult :type Hit%20Result%20Structure%20%28by%20ref%29))
  ;[1 1 1] A porte
  (Variables|Default|SetInBox true)
  (Rendering|SetVisibility (Variables|Default|GetinteractIcon) true false))

(event OnComponentEndOverlap(Box)
  (params (OverlappedComponent :type Primitive%20Component%20Object%20Reference) (OtherActor :type Actor%20Object%20Reference) (OtherComp :type Primitive%20Component%20Object%20Reference) (OtherBodyIndex :type Integer))
  ;[1 1 1] A porte
  (Variables|Default|SetInBox false)
  (Rendering|SetVisibility (Variables|Default|GetinteractIcon) false false))

(event EventBeginPlay
  (Variables|Default|SetRefPlayer (.AsBP%20First%20Person%20Character (Utilities|Casting|CastToBP_FirstPersonCharacter (Game|GetPlayerCharacter 0)))))

(event Collision|EventActorBeginOverlap
  (params (OtherActor :type Actor%20Object%20Reference)))

(event EventTick
  (params (DeltaSeconds :type Float%20%28single-precision%29)))

(event EventInteraction
  (bind _refplayer (Variables|Default|GetRefPlayer))
  (bind _returnvalue (UserInterface|CreateWidget "/Game/Widget/WG_TexteLore.WG_TexteLore_C" 0 (Variables|Default|GetIDTexte)))
  (UserInterface|Viewport|AddtoViewport _returnvalue 0)
  (Variables|/Game/FirstPerson/Blueprints/BP_FirstPersonCharacter.BP_FirstPersonCharacter_C|SetCanMove _refplayer false)
  (Variables|/Game/FirstPerson/Blueprints/BP_FirstPersonCharacter.BP_FirstPersonCharacter_C|SetCanLook _refplayer false)
  (Variables|/Game/FirstPerson/Blueprints/BP_FirstPersonCharacter.BP_FirstPersonCharacter_C|SetCanPower _refplayer false)
  (Variables|/Game/FirstPerson/Blueprints/BP_FirstPersonCharacter.BP_FirstPersonCharacter_C|SetCanInteract _refplayer false))

(fn ConstructionScript)
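; Candle prop with a selectable mesh and a flame that turns to face the player's first-person camera.
; The construction script uses Id to pick the candle mesh from MeshToUse and set the flame's height and scale to match.
; Box overlap with BP_FirstPersonCharacter toggles BOugieTurn, so Tick billboards the flame only while the player is inside.
; The billboard takes yaw and roll from a look-at rotation with 90-degree offsets, holding pitch at zero.
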(event OnComponentBeginOverlap(Box)
  (params (OverlappedComponent :type Primitive%20Component%20Object%20Reference) (OtherActor :type Actor%20Object%20Reference) (OtherComp :type Primitive%20Component%20Object%20Reference) (OtherBodyIndex :type Integer) (bFromSweep :type Boolean) (SweepResult :type Hit%20Result%20Structure%20%28by%20ref%29))
  (Utilities|Casting|CastToBP_FirstPersonCharacter OtherActor)
  (Variables|Default|SetBOugieTurn true))

(event OnComponentEndOverlap(Box)
  (params (OverlappedComponent :type Primitive%20Component%20Object%20Reference) (OtherActor :type Actor%20Object%20Reference) (OtherComp :type Primitive%20Component%20Object%20Reference) (OtherBodyIndex :type Integer))
  (Utilities|Casting|CastToBP_FirstPersonCharacter OtherActor)
  (Variables|Default|SetBOugieTurn false))

(event EventBeginPlay)

(event Collision|EventActorBeginOverlap
  (params (OtherActor :type Actor%20Object%20Reference)))

(event EventTick
  (params (DeltaSeconds :type Float%20%28single-precision%29))
  (bind _returnvalue (Game|GetPlayerCharacter 0))
  (bind _flamme (Variables|Default|GetFlamme))
  (bind _returnvalue_2 (Transformation|GetWorldLocation _flamme))
  (bind _asbp_first_person_character (Utilities|Casting|CastToBP_FirstPersonCharacter _returnvalue))
  (bind _firstpersoncamera (Variables|/Game/FirstPerson/Blueprints/BP_FirstPersonCharacter.BP_FirstPersonCharacter_C|GetFirstPersonCamera _asbp_first_person_character))
  (bind _returnvalue_3 (Transformation|GetWorldLocation _firstpersoncamera))
  (bind _returnvalue_4 (Math|Rotator|FindLookatRotation _returnvalue_2 _returnvalue_3))
  (if (Variables|Default|GetBOugieTurn)
    (Transformation|SetWorldRotation (Variables|Default|GetFlamme) (Math|Rotator|MakeRotator (+ (.roll _returnvalue_4) 9e+01) 0.0 (+ (.yaw _returnvalue_4) -9e+01)) false false)))

(fn ConstructionScript
  (bind _flamme (Variables|Default|GetFlamme))
  (bind _flamme_2 (Variables|Default|GetFlamme))
  (bind _flamme_3 (Variables|Default|GetFlamme))
  (bind _flamme_4 (Variables|Default|GetFlamme))
  (switch int (Variables|Default|GetId)
    (:0
      (Transformation|SetRelativeLocation _flamme_3 "0.000000,0.000000,25.000000" false false)
      (Transformation|SetRelativeScale3D _flamme_3 "0.050000,0.170000,0.170000")
      (Components|StaticMesh|SetStaticMesh (Variables|Default|GetBougie%20Grande) (Utilities|Array|Get(acopy) (Variables|Default|GetMeshToUse) (Variables|Default|GetId))))
    (:1
      (Transformation|SetRelativeLocation _flamme_4 "0.000000,0.000000,17.000000" false false)
      (Transformation|SetRelativeScale3D _flamme_4 "0.050000,0.170000,0.170000")
      (Components|StaticMesh|SetStaticMesh (Variables|Default|Getbougie_Grande) (Utilities|Array|Get(acopy) (Variables|Default|GetMeshToUse) (Variables|Default|GetId))))
    (:2
      (Transformation|SetRelativeLocation _flamme "0.000000,0.000000,12.000000" false false)
      (Transformation|SetRelativeScale3D _flamme "0.050000,0.170000,0.170000")
      (Components|StaticMesh|SetStaticMesh (Variables|Default|Getbougie_Grande) (Utilities|Array|Get(acopy) (Variables|Default|GetMeshToUse) (Variables|Default|GetId))))
    (:3
      (Transformation|SetRelativeLocation _flamme_2 "0.000000,0.000000,68.000000" false false)
      (Transformation|SetRelativeScale3D _flamme_2 "0.160000,0.570000,0.170000")
      (Components|StaticMesh|SetStaticMesh (Variables|Default|Getbougie_Grande) (Utilities|Array|Get(acopy) (Variables|Default|GetMeshToUse) (Variables|Default|GetId))))))
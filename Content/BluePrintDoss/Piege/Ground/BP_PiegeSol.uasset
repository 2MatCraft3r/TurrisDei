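; BP_PiegeSol is an animated ground trap that sends the first-person player back to their respawn point on contact.
; Each Tick, the Box hit volume follows a socket on GroundTrapANIM with a downward offset.
; Touching the Box plays a death fade on the player's transition widget, teleporting the capsule to ReSpawn between delays.
; A separate Detection volume sets an in-range flag and starts or stops the trap sound.
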(event OnComponentBeginOverlap(Box)
  (params (OverlappedComponent :type Primitive%20Component%20Object%20Reference) (OtherActor :type Actor%20Object%20Reference) (OtherComp :type Primitive%20Component%20Object%20Reference) (OtherBodyIndex :type Integer) (bFromSweep :type Boolean) (SweepResult :type Hit%20Result%20Structure%20%28by%20ref%29))
  (bind _returnvalue (Game|GetPlayerCharacter 0))
  (bind _asbp_first_person_character (Utilities|Casting|CastToBP_FirstPersonCharacter _returnvalue))
  (bind _reftransi (Variables|/Game/FirstPerson/Blueprints/BP_FirstPersonCharacter.BP_FirstPersonCharacter_C|GetRefTransi _asbp_first_person_character))
  (if (== OtherActor _asbp_first_person_character)
    (Widget|SetVisibility _reftransi "Visible")
    (Default|FadeMorte _reftransi)
    (Utilities|FlowControl|Delay 0.5)
    (Transformation|SetWorldTransform (Variables|/Script/Engine.Character|GetCapsuleComponent _asbp_first_person_character) (Variables|/Game/FirstPerson/Blueprints/BP_FirstPersonCharacter.BP_FirstPersonCharacter_C|GetReSpawn _asbp_first_person_character) false false)
    (Utilities|FlowControl|Delay 0.5)
    (Default|FadeEnd _reftransi)))

(event OnComponentBeginOverlap(Detection)
  (params (OverlappedComponent :type Primitive%20Component%20Object%20Reference) (OtherActor :type Actor%20Object%20Reference) (OtherComp :type Primitive%20Component%20Object%20Reference) (OtherBodyIndex :type Integer) (bFromSweep :type Boolean) (SweepResult :type Hit%20Result%20Structure%20%28by%20ref%29))
  (bind _piegeeffect (Variables|Default|GetPiegeEffect))
  (if (== OtherActor (Game|GetPlayerCharacter 0))
    (Variables|Default|SetAPortye true)
    (Audio|Components|Audio|SetVolumeMultiplier _piegeeffect 1.0 :!class /Script/Engine.AudioComponent)
    (Audio|Components|Audio|Play _piegeeffect 0.0)))

(event OnComponentEndOverlap(Detection)
  (params (OverlappedComponent :type Primitive%20Component%20Object%20Reference) (OtherActor :type Actor%20Object%20Reference) (OtherComp :type Primitive%20Component%20Object%20Reference) (OtherBodyIndex :type Integer))
  (if (== OtherActor (Game|GetPlayerCharacter 0))
    (Variables|Default|SetAPortye false)
    (Audio|Components|Audio|Stop (Variables|Default|GetPiegeEffect))))

(event EventBeginPlay)

(event Collision|EventActorBeginOverlap
  (params (OtherActor :type Actor%20Object%20Reference)))

(event EventTick
  (params (DeltaSeconds :type Float%20%28single-precision%29))
  (Transformation|SetWorldLocation (Variables|Default|GetBox) (- (Transformation|GetSocketLocation (Variables|Default|GetGround_Trap_ANIM) "pasted__pCube2") "0.000000,0.000000,30.000000") false false))

(fn ConstructionScript)
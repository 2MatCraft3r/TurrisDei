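; AI controller for the final SCP monster, running its behavior tree and hunting the player by sight.
; Player spell events toggle the sight sense, which starts disabled; re-enabling it can also flag tutorial success on the blackboard.
; SensVue writes the seen player or last known position to the blackboard, switching between chase and slower speeds.
; A player tutorial event spawns a separate scripted monster and sets its blackboard destination.
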(event Custom|Enlever
  ;[1 1 1] EteindreLight
  (Class|AIPerceptionComponent|SetSenseEnabled (Class|AIController|GetAIPerceptionComponent) "/Script/AIModule.AISense_Sight" false))

(event Custom|MettreVue
  ;[1 1 1] LightAllumer
  (Class|AIPerceptionComponent|SetSenseEnabled (Class|AIController|GetAIPerceptionComponent) "/Script/AIModule.AISense_Sight" true)
  (if (Variables|/Game/FirstPerson/Blueprints/BP_FirstPersonCharacter.BP_FirstPersonCharacter_C|GetScpTutoAllume (Variables|Default|GetPlayerRef))
    (AI|Components|Blackboard|SetValueasBool (AI|GetBlackboard self) (Utilities|Name|MakeLiteralName "QteTutoReussit") true)
    (Default|CallSetSpeed 1.5e+02)
    (Audio|PlaySound2D "/Engine/EditorSounds/GamePreview/EndPlayInEditor.EndPlayInEditor" 1.0 1.0 0.0 0 0)))

(event Custom|Tuto
  (params (SpawnMonstre :type Actor%20Object%20Reference) (NewParam :type Actor%20Object%20Reference))
  ;[1 1 1] TutoSCP
  (Development|PrintString "Spawn")
  (bind _returnvalue (Game|SpawnActorfromClass "/Game/BluePrintDoss/IAMOnstre/ScriptTutoMonstre/BP_MonstreTuto.BP_MonstreTuto_C" (Transformation|GetActorTransform SpawnMonstre) "Undefined" "MultiplyWithRoot" 0 0))
  (Variables|Default|SetMonstreTuto _returnvalue)
  (Utilities|FlowControl|Delay 0.5)
  (AI|Components|Blackboard|SetValueasBool (AI|GetBlackboard _returnvalue) (Utilities|Name|MakeLiteralName "ScriptTuto") true)
  (AI|Components|Blackboard|SetValueasVector (AI|GetBlackboard _returnvalue) (Utilities|Name|MakeLiteralName "NewLocation") (Transformation|GetActorLocation NewParam)))

(event EventBeginPlay
  ;[0.0226 1 0] BeginPlay
  (Utilities|FlowControl|Sequence
    (:then_0
      (AI|RunBehaviorTree "/Game/BluePrintDoss/IAMOnstre/SCPMostre_Fin/BT_MonstreFin.BT_MonstreFin")
      (Class|AIPerceptionComponent|SetSenseEnabled (Class|AIController|GetAIPerceptionComponent) "/Script/AIModule.AISense_Sight" false)
      (bind _asbp_first_person_character (Utilities|Casting|CastToBP_FirstPersonCharacter (Game|GetPlayerCharacter 0)))
      (Variables|Default|SetPlayerRef _asbp_first_person_character))
    (:then_1
      (EventDispatchers|BindEventtoSort1Valid (Variables|Default|GetPlayerRef) (delegate Custom|Enlever))
      (EventDispatchers|BindEventtoSort2Valid (Variables|Default|GetPlayerRef) (delegate Custom|MettreVue))
      (EventDispatchers|BindEventtoScriptTutoLink (Variables|Default|GetPlayerRef) (delegate Custom|Tuto)))))

(event EventTick
  (params (DeltaSeconds :type Float%20%28single-precision%29)))

(fn ConstructionScript)

(fn SensVue
  (params (Actor :type Actor%20Object%20Reference) (Stimullus :type AI%20Stimulus%20Structure))
  (bind _returnvalue (Class|AIPerceptionSystem|GetSenseClassforStimulus Stimullus))
  (if (== _returnvalue "/Script/AIModule.AISense_Sight")
    (if (== Actor (Game|GetPlayerCharacter 0))
      (if (.bsuccessfullysensed Stimullus)
        (bind _output_get (Variables|Default|SetMonstreVoit true))
        (AI|Components|Blackboard|SetValueasObject (Variables|Default|GetBlackboard) (Utilities|Name|MakeLiteralName "PlayerRef") (Utilities|SelectObject (Game|GetPlayerCharacter 0) 0 _output_get))
        (Default|CallSetSpeed 6e+02)
        (else
          (Variables|Default|SetMonstreVoit false)
          (AI|Components|Blackboard|SetValueasVector (Variables|Default|GetBlackboard) (Utilities|Name|MakeLiteralName "LastPlayerPosition") (.stimuluslocation Stimullus))
          (Variables|Default|SetViensDePlusVoir true)
          (AI|Components|Blackboard|SetValueasObject (Variables|Default|GetBlackboard) (Utilities|Name|MakeLiteralName "PlayerRef") (Utilities|SelectObject (Game|GetPlayerCharacter 0) 0 false))
          (Default|CallSetSpeed 1.5e+02)))
      (else
        (return)))
    (else
      (return))))
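; BP_TutoActive is a one-shot trigger actor that shows the tutorial widget when the player leaves its ActiveTuto component.
; On BeginPlay it creates WG_Tuto, adds it to the viewport and hides it.
; When the player character's overlap ends, provided Activable and the first-time flag are set, it clears the flag.
; After a short delay it reveals the widget, shows the cursor and switches input to UI-only.
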(event OnComponentEndOverlap(ActiveTuto)
  (params (OverlappedComponent :type Primitive%20Component%20Object%20Reference) (OtherActor :type Actor%20Object%20Reference) (OtherComp :type Primitive%20Component%20Object%20Reference) (OtherBodyIndex :type Integer))
  (bind _returnvalue (Game|GetPlayerController 0))
  (bind _reftuto (Variables|Default|GetrefTuto))
  (if (Variables|Default|GetActivable)
    (if (and (Variables|Default|GetpremeireFois) (== OtherActor (.AsBP%20First%20Person%20Character (Utilities|Casting|CastToBP_FirstPersonCharacter (Game|GetPlayerCharacter 0)))))
      (Variables|Default|SetpremeireFois false)
      (Utilities|FlowControl|Delay 1.0)
      (Widget|SetVisibility _reftuto "Visible")
      (Variables|/Script/Engine.PlayerController|SetbShowMouseCursor _returnvalue true)
      (Input|SetInputModeUIOnly _returnvalue _reftuto "DoNotLock" false))))

(event EventBeginPlay
  (bind _returnvalue (UserInterface|CreateWidget "/Game/Widget/WG_Tuto.WG_Tuto_C"))
  (bind _output_get (Variables|Default|SetrefTuto _returnvalue))
  (UserInterface|Viewport|AddtoViewport _output_get 0)
  (Widget|SetVisibility _output_get "Hidden"))

(event Collision|EventActorBeginOverlap
  (params (OtherActor :type Actor%20Object%20Reference)))

(event EventTick
  (params (DeltaSeconds :type Float%20%28single-precision%29)))

(fn ConstructionScript)
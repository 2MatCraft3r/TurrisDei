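; BP_CamCineFin is a camera view-target actor, apparently for an ending cinematic tied to the player's SCPFin event.
; On BeginPlay it caches the BP_FirstPersonCharacter and binds its SCPFInCam handler to that character's SCPFin event.
; When fired, the handler blends the player controller's view to this actor, waits out the blend, then calls SCPFinSort on the character.
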(event Custom|SCPFInCam
  (Game|Player|SetViewTargetwithBlend (Game|GetPlayerController 0) self 2.0 "VTBlend_Linear" 0.0 false)
  (Utilities|FlowControl|Delay 2.0)
  (Default|SCPFinSort (Variables|Default|GetRefPlayer)))

(event EventBeginPlay
  (bind _asbp_first_person_character (Utilities|Casting|CastToBP_FirstPersonCharacter (Game|GetPlayerCharacter 0)))
  (bind _output_get (Variables|Default|SetRefPlayer _asbp_first_person_character))
  (EventDispatchers|BindEventtoSCPFin _output_get (delegate Custom|SCPFInCam)))

(event Collision|EventActorBeginOverlap
  (params (OtherActor :type Actor%20Object%20Reference)))

(event EventTick
  (params (DeltaSeconds :type Float%20%28single-precision%29)))

(fn ConstructionScript)
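; BP_FeuilleFinal is an interactable actor, apparently the final sheet, that brings up the WG_Fin end screen.
; On BeginPlay it creates the widget, adds it to the viewport and keeps it hidden.
; Its Interaction event reveals the widget, hides the static mesh, shows the mouse cursor and switches input to UI-only focused on the widget.
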(event EventBeginPlay
  (bind _returnvalue (UserInterface|CreateWidget "/Game/Widget/WG_Fin.WG_Fin_C"))
  (bind _output_get (Variables|Default|SetRefFIn _returnvalue))
  (UserInterface|Viewport|AddtoViewport _output_get 0)
  (Widget|SetVisibility _output_get "Hidden"))

(event Collision|EventActorBeginOverlap
  (params (OtherActor :type Actor%20Object%20Reference)))

(event EventTick
  (params (DeltaSeconds :type Float%20%28single-precision%29)))

(event EventInteraction
  (bind _returnvalue (Game|GetPlayerController 0))
  (bind _reffin (Variables|Default|GetRefFIn))
  (Utilities|FlowControl|Sequence
    (:then_0
      (Widget|SetVisibility _reffin "Visible")
      (Development|SetHiddeninGame (Variables|Default|GetStaticMesh) true false)
      (Variables|/Script/Engine.PlayerController|SetbShowMouseCursor _returnvalue true)
      (Input|SetInputModeUIOnly _returnvalue _reffin "DoNotLock" false))))

(fn ConstructionScript)
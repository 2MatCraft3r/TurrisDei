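; BP_CamFinal is the ending camera that takes over the view for the game's final cinematic.
; On BeginPlay it hides the Habit actor and binds SwitchCamFinal to an event on the first-person character.
; When that fires, it blends the player's view to itself and reveals Habit.
; After timed delays it runs a fade transition through the player's RefTransi widget, then shows and starts the RefCineFin ending cinematic.
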(event Custom|SwitchCamFinal
  (bind _refplayer (Variables|Default|GetrefPlayer))
  (bind _reftransi (Variables|/Game/FirstPerson/Blueprints/BP_FirstPersonCharacter.BP_FirstPersonCharacter_C|GetRefTransi _refplayer))
  (bind _refcinefin (Variables|/Game/FirstPerson/Blueprints/BP_FirstPersonCharacter.BP_FirstPersonCharacter_C|GetRefCineFin _refplayer))
  (Game|Player|SetViewTargetwithBlend (Game|GetPlayerController 0) self 2.0 "VTBlend_Linear" 0.0 false)
  (Rendering|SetActorHiddenInGame (Variables|Default|GetHabit) false)
  (Utilities|FlowControl|Delay 4.0)
  (Widget|SetVisibility _reftransi "Visible")
  (Default|FadeNoir _reftransi)
  (Utilities|FlowControl|Delay 0.5)
  (Default|FadeEnd _reftransi)
  (Widget|SetVisibility _refcinefin "Visible")
  (Default|StatFin _refcinefin))

(event EventBeginPlay
  (bind _output_get (Variables|Default|SetrefPlayer (.AsBP%20First%20Person%20Character (Utilities|Casting|CastToBP_FirstPersonCharacter (Game|GetPlayerCharacter 0)))))
  (EventDispatchers|BindEventtoCamFinFin _output_get (delegate Custom|SwitchCamFinal))
  (Rendering|SetActorHiddenInGame (Variables|Default|GetHabit) true))

(event Collision|EventActorBeginOverlap
  (params (OtherActor :type Actor%20Object%20Reference)))

(event EventTick
  (params (DeltaSeconds :type Float%20%28single-precision%29)))

(fn ConstructionScript)
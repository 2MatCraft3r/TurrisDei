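; AI controller for the monster of a scripted corridor sequence, running BT_MonstreScript1 with sight initially disabled.
; Player character events toggle sight (spell 1 off, spell 2 on), spawn the monster and send it toward a target, or hand it the player on QTE failure.
; SensVue turns sight stimuli into blackboard player or last-seen position, switching between chase and slower speeds.
; Re-enabling sight can also flag tutorial QTE success and trigger a cry.
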(event Custom|SpawnAndMoove
  (params (SpawnMonstre :type Actor%20Object%20Reference) (NewParam :type Actor%20Object%20Reference))
  ;[0 1 0.1157] Script1
  (Development|PrintString "Hello")
  (bind _returnvalue (Game|SpawnActorfromClass "/Game/BluePrintDoss/IAMonstre/ScriptCouloirMonstre/BP_MonstreScript1.BP_MonstreScript1_C" (Transformation|GetActorTransform SpawnMonstre) "Undefined" "MultiplyWithRoot" 0 0))
  (Variables|Default|SetRefMonstre _returnvalue)
  (Utilities|FlowControl|Delay 0.2)
  (AI|Components|Blackboard|SetValueasBool (AI|GetBlackboard _returnvalue) (Utilities|Name|MakeLiteralName "Sript1") true)
  (AI|Components|Blackboard|SetValueasVector (AI|GetBlackboard _returnvalue) (Utilities|Name|MakeLiteralName "NewLocation") (Transformation|GetActorLocation NewParam))
  (Default|CallSetSpeed 2e+01)
  (Class|AIPerceptionComponent|SetSenseEnabled (Class|AIController|GetAIPerceptionComponent) "/Script/AIModule.AISense_Sight" false))

(event Custom|QTERaterSCP1
  ;[1 1 1] Script1Faild
  (AI|Components|Blackboard|SetValueasObject (AI|GetBlackboard self) (Utilities|Name|MakeLiteralName "PlayerRef") (Variables|Default|GetPlayerRef)))

(event Custom|Enlever
  ;[1 1 1] EteindreLight
  (Class|AIPerceptionComponent|SetSenseEnabled (Class|AIController|GetAIPerceptionComponent) "/Script/AIModule.AISense_Sight" false))

(event Custom|MettreVue
  ;[1 1 1] LightAllumer
  (Class|AIPerceptionComponent|SetSenseEnabled (Class|AIController|GetAIPerceptionComponent) "/Script/AIModule.AISense_Sight" true)
  (if (Variables|/Game/FirstPerson/Blueprints/BP_FirstPersonCharacter.BP_FirstPersonCharacter_C|GetScpTutoAllume (.AsBP%20First%20Person%20Character (Utilities|Casting|CastToBP_FirstPersonCharacter (Game|GetPlayerCharacter 0))))
    (AI|Components|Blackboard|SetValueasBool (AI|GetBlackboard (Variables|Default|GetMonstreTuto)) (Utilities|Name|MakeLiteralName "QteTutoReussit") true)
    (Default|CallSetSpeed 1.5e+02)
    (Default|CallCri)))

(event EventBeginPlay
  (bind _returnvalue (Game|GetPlayerCharacter 0))
  (bind _asbp_first_person_character (Utilities|Casting|CastToBP_FirstPersonCharacter _returnvalue))
  ;[0.0226 1 0] BeginPlay
  (Utilities|FlowControl|Sequence
    (:then_0
      (AI|RunBehaviorTree "/Game/BluePrintDoss/IAMonstre/ScriptCouloirMonstre/BT_MonstreScript1.BT_MonstreScript1")
      (Class|AIPerceptionComponent|SetSenseEnabled (Class|AIController|GetAIPerceptionComponent) "/Script/AIModule.AISense_Sight" false)
      (bind _asbp_first_person_character_2 (Utilities|Casting|CastToBP_FirstPersonCharacter (Game|GetPlayerCharacter 0)))
      (Variables|Default|SetPlayerRef _asbp_first_person_character_2))
    (:then_1
      (EventDispatchers|BindEventtoSort1Valid _asbp_first_person_character (delegate Custom|Enlever))
      (EventDispatchers|BindEventtoSort2Valid _asbp_first_person_character (delegate Custom|MettreVue))
      (EventDispatchers|BindEventtoScript01 _asbp_first_person_character (delegate Custom|SpawnAndMoove))
      (EventDispatchers|BindEventtoSCP1Fail _asbp_first_person_character (delegate Custom|QTERaterSCP1)))))

(event EventTick
  (params (DeltaSeconds :type Float%20%28single-precision%29)))

(fn ConstructionScript)

(fn SensVue
  (params (Actor :type Actor%20Object%20Reference) (Stimullus :type AI%20Stimulus%20Structure))
  (bind _returnvalue (Class|AIPerceptionSystem|GetSenseClassforStimulus Stimullus))
  (if (== _returnvalue "/Script/AIModule.AISense_Sight")
    (if (== Actor (Game|GetPlayerCharacter 0))
      (if (.bsuccessfullysensed Stimullus)
        (bind _output_get (Variables|Default|SetMonstreVoit true))
        (AI|Components|Blackboard|SetValueasObject (Variables|Default|GetBlackboard) (Utilities|Name|MakeLiteralName "PlayerRef") (Utilities|SelectObject (Game|GetPlayerCharacter 0) 0 _output_get))
        (Default|CallSetSpeed 6e+02)
        (else
          (Variables|Default|SetMonstreVoit false)
          (AI|Components|Blackboard|SetValueasVector (Variables|Default|GetBlackboard) (Utilities|Name|MakeLiteralName "LastPlayerPosition") (.stimuluslocation Stimullus))
          (Variables|Default|SetViensDePlusVoir true)
          (AI|Components|Blackboard|SetValueasObject (Variables|Default|GetBlackboard) (Utilities|Name|MakeLiteralName "PlayerRef") (Utilities|SelectObject (Game|GetPlayerCharacter 0) 0 false))
          (Default|CallSetSpeed 1.5e+02)))
      (else
        (return)))
    (else
      (return))))
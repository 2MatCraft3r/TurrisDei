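; BP_Monstre is a monster character that reacts to the player's two spells and sends the player back to respawn on contact.
; On BeginPlay it binds Ralntir and Stunn to the first-person character's Sort1Valid and Sort2Valid events.
; These temporarily slow or stop its walking through MaxWalkSpeed and a Delay.
; Overlapping its ZoneDemort component teleports the player's capsule to their stored ReSpawn transform.
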(event OnComponentBeginOverlap(ZoneDemort)
  (params (OverlappedComponent :type Primitive%20Component%20Object%20Reference) (OtherActor :type Actor%20Object%20Reference) (OtherComp :type Primitive%20Component%20Object%20Reference) (OtherBodyIndex :type Integer) (bFromSweep :type Boolean) (SweepResult :type Hit%20Result%20Structure%20%28by%20ref%29))
  (bind _asbp_first_person_character (Utilities|Casting|CastToBP_FirstPersonCharacter OtherActor))
  (Transformation|SetWorldTransform (Variables|/Script/Engine.Character|GetCapsuleComponent _asbp_first_person_character) (Variables|/Game/FirstPerson/Blueprints/BP_FirstPersonCharacter.BP_FirstPersonCharacter_C|GetReSpawn _asbp_first_person_character) false false))

(event Custom|Ralntir
  (bind _charactermovement (Variables|Character|GetCharacterMovement))
  (Development|PrintString "rallentuss" true true "(R=1.000000,G=0.000000,B=0.264599,A=1.000000)")
  (Variables|/Script/Engine.CharacterMovementComponent|SetMaxWalkSpeed _charactermovement 2e+02)
  (Utilities|FlowControl|Delay 2.0)
  (Variables|/Script/Engine.CharacterMovementComponent|SetMaxWalkSpeed _charactermovement 4e+02))

(event Custom|Stunn
  (bind _charactermovement (Variables|Character|GetCharacterMovement))
  (Development|PrintString "stun")
  (Variables|/Script/Engine.CharacterMovementComponent|SetMaxWalkSpeed _charactermovement 0.0)
  (Utilities|FlowControl|Delay 1e+01)
  (Variables|/Script/Engine.CharacterMovementComponent|SetMaxWalkSpeed _charactermovement 4e+02))

(event EventBeginPlay
  (bind _asbp_first_person_character (Utilities|Casting|CastToBP_FirstPersonCharacter (Game|GetPlayerCharacter 0)))
  (EventDispatchers|BindEventtoSort1Valid _asbp_first_person_character (delegate Custom|Ralntir))
  (EventDispatchers|BindEventtoSort2Valid _asbp_first_person_character (delegate Custom|Stunn)))

(event Collision|EventActorBeginOverlap
  (params (OtherActor :type Actor%20Object%20Reference)))

(event EventTick
  (params (DeltaSeconds :type Float%20%28single-precision%29)))

(fn ConstructionScript)
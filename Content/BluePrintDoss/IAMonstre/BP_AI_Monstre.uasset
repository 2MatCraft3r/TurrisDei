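; AI controller for the monster, which runs BT_Monstre and hunts the player by sight.
; Sight starts disabled and is toggled by two player spell events, with switch-off also clearing the blackboard target.
; Perception updates set PlayerRef and raise speed when the player is seen, or clear it, store the last known position and slow down when lost.
; A separate CriMonstre event plays the monster's scream sound.
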(event OnTargetPerceptionUpdated(Vue)
  (params (Actor :type Actor%20Object%20Reference) (Stimulus :type AI%20Stimulus%20Structure))
  ;[0 1 0.08263] A cahque fois qu'il voit / voit plus ca lance la fonction Sens vue
  (CallFunction|SensVue Actor Stimulus))

(event Custom|Enlever
  ;[1 1 1] EteindreLight
  (Class|AIPerceptionComponent|SetSenseEnabled (Class|AIController|GetAIPerceptionComponent) "/Script/AIModule.AISense_Sight" false)
  (CallFunction|Cacher))

(event Custom|MettreVue
  ;[1 1 1] LightAllumer
  (Class|AIPerceptionComponent|SetSenseEnabled (Class|AIController|GetAIPerceptionComponent) "/Script/AIModule.AISense_Sight" true))

(event Custom|Cacher
  ;[0 1 0.01945] Quand ON eteins le livre ca enleve la ref du player
  (AI|Components|Blackboard|SetValueasObject (Variables|Default|GetBlackboard) (Utilities|Name|MakeLiteralName "PlayerRef") 0)
  (Default|CallSetSpeed 1.5e+02))

(event Custom|CriMonstre
  ;[1 1 1] Quand le Monstre Voit le Player Lance Cri
  (Variables|Default|SetMonstreCri (ScalableFloat|GetValueasBool (Variables|Default|GetBlackboard) (Utilities|Name|MakeLiteralName "CanCri")))
  (Audio|Components|Audio|Play (Variables|/Game/BluePrintDoss/IAMOnstre/BP_Monstre.BP_Monstre_C|Getcri_Donatien_lent_puissant1_25sec (Variables|Default|GetMonstreReff)) 0.0)
  (Utilities|FlowControl|Delay 1.25)
  (Variables|Default|SetMonstreCri false))

(event EventBeginPlay
  (bind _returnvalue (Game|GetPlayerCharacter 0))
  (bind _asbp_first_person_character (Utilities|Casting|CastToBP_FirstPersonCharacter _returnvalue))
  ;[0.0226 1 0] BeginPlay
  (Utilities|FlowControl|Sequence
    (:then_0
      (AI|RunBehaviorTree "/Game/BluePrintDoss/IAMOnstre/BT_Monstre.BT_Monstre")
      (Class|AIPerceptionComponent|SetSenseEnabled (Class|AIController|GetAIPerceptionComponent) "/Script/AIModule.AISense_Sight" false)
      (Utilities|Casting|CastToBP_FirstPersonCharacter (Game|GetPlayerCharacter 0))
      (Variables|Default|SetPlayerRef 0))
    (:then_1
      (EventDispatchers|BindEventtoSort1Valid _asbp_first_person_character (delegate Custom|Enlever))
      (EventDispatchers|BindEventtoSort2Valid _asbp_first_person_character (delegate Custom|MettreVue)))))

(event EventTick
  (params (DeltaSeconds :type Float%20%28single-precision%29)))

(fn ConstructionScript)

(fn SensVue
  (params (Actor :type Actor%20Object%20Reference) (Stimullus :type AI%20Stimulus%20Structure))
  (bind _returnvalue (Class|AIPerceptionSystem|GetSenseClassforStimulus Stimullus))
  (if (== _returnvalue "/Script/AIModule.AISense_Sight")
    (if (== Actor (Game|GetPlayerCharacter 0))
      (if (.bsuccessfullysensed Stimullus)
        (bind _output_get (Variables|Default|SetMonstreVoit true))
        (AI|Components|Blackboard|SetValueasObject (Variables|Default|GetBlackboard) (Utilities|Name|MakeLiteralName "PlayerRef") (Utilities|SelectObject (Game|GetPlayerCharacter 0) 0 _output_get))
        (Default|CallSetSpeed 6e+02)
        (else
          (Variables|Default|SetMonstreVoit false)
          (AI|Components|Blackboard|SetValueasVector (Variables|Default|GetBlackboard) (Utilities|Name|MakeLiteralName "LastPlayerPosition") (.stimuluslocation Stimullus))
          (Variables|Default|SetViensDePlusVoir true)
          (AI|Components|Blackboard|SetValueasObject (Variables|Default|GetBlackboard) (Utilities|Name|MakeLiteralName "PlayerRef") (Utilities|SelectObject (Game|GetPlayerCharacter 0) 0 false))
          (Default|CallSetSpeed 1.5e+02)))
      (else
        (return)))
    (else
      (return))))
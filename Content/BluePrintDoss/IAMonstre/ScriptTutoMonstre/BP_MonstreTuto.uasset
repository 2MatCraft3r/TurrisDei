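; BP_MonstreTuto is the tutorial monster character that sends the player back to a respawn point on contact.
; It takes speed changes from its BP_AI_MonstreTuto controller and destroys itself when the player's destroy event fires.
; Overlapping ZoneDemort teleports the player's capsule to ReSpawn while a brief death shot switches the view to the lit-up monster.
; After a short delay, the view returns to the player and the transition's FadeEnd runs.
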(event OnComponentBeginOverlap(ZoneDemort)
  (params (OverlappedComponent :type Primitive%20Component%20Object%20Reference) (OtherActor :type Actor%20Object%20Reference) (OtherComp :type Primitive%20Component%20Object%20Reference) (OtherBodyIndex :type Integer) (bFromSweep :type Boolean) (SweepResult :type Hit%20Result%20Structure%20%28by%20ref%29))
  (bind _playerref (Variables|Default|GetPLayerRef))
  ;[0 1 0.1098] MortCollision
  (if (== OtherActor _playerref)
    (Transformation|SetWorldTransform (Variables|/Script/Engine.Character|GetCapsuleComponent _playerref) (Variables|/Game/FirstPerson/Blueprints/BP_FirstPersonCharacter.BP_FirstPersonCharacter_C|GetReSpawn _playerref) false false)
    (Game|Player|SetViewTargetwithBlend (Game|GetPlayerController 0) self 0.0 "VTBlend_Linear" 0.0 false)
    (Variables|Default|SetMortActive true)
    (Rendering|Components|Light|SetIntensity (Variables|Default|GetSpotLight) 6.5e+02)
    (Utilities|FlowControl|Delay 0.8)
    (Game|Player|SetViewTargetwithBlend (Game|GetPlayerController 0) (Game|GetPlayerCharacter 0) 0.0 "VTBlend_Linear" 0.0 false)
    (Default|FadeEnd (Variables|/Game/FirstPerson/Blueprints/BP_FirstPersonCharacter.BP_FirstPersonCharacter_C|GetRefTransi (Variables|Default|GetPLayerRef)))
    (Variables|Default|SetMortActive false)
    (Rendering|Components|Light|SetIntensity (Variables|Default|GetSpotLight) 0.0)))

(event Custom|SetLaSpeed
  (params (CurrentSpeed :type Float%20%28double-precision%29))
  ;[0.04481 1 0] BeginPlay
  (Variables|/Script/Engine.CharacterMovementComponent|SetMaxWalkSpeed (Variables|Character|GetCharacterMovement) CurrentSpeed))

(event Custom|Destroy
  ;[0.04481 1 0] BeginPlay
  (Actor|DestroyActor))

(event EventBeginPlay
  ;[0.04481 1 0] BeginPlay
  (bind _asbp_ai_monstre_tuto (Utilities|Casting|CastToBP_AI_MonstreTuto (AI|GetAIController self)))
  (EventDispatchers|BindEventtoSetSpeed _asbp_ai_monstre_tuto (delegate Custom|SetLaSpeed))
  (Variables|/Script/Engine.CharacterMovementComponent|SetMaxWalkSpeed (Variables|Character|GetCharacterMovement) 1.5e+02)
  (bind _asbp_first_person_character (Utilities|Casting|CastToBP_FirstPersonCharacter (Game|GetPlayerCharacter 0)))
  (bind _output_get (Variables|Default|SetPLayerRef _asbp_first_person_character))
  (EventDispatchers|BindEventtoDestroyMonstre _output_get (delegate Custom|Destroy)))

(event Collision|EventActorBeginOverlap
  (params (OtherActor :type Actor%20Object%20Reference)))

(fn ConstructionScript)
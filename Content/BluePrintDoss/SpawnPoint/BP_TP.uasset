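; BP_TP is a teleport trigger that moves the player between rooms using level streaming.
; On overlap it fades to black through a WG_TransiTP widget created at BeginPlay, then switches on IdTp to pick the destination room.
; Each case loads that streamed level, teleports the player to LieuxTP, then unloads neighboring rooms after a delay.
; FadeEnd runs from a parallel Sequence pin, without waiting for loading to finish.
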(event OnComponentBeginOverlap(TP)
  (params (OverlappedComponent :type Primitive%20Component%20Object%20Reference) (OtherActor :type Actor%20Object%20Reference) (OtherComp :type Primitive%20Component%20Object%20Reference) (OtherBodyIndex :type Integer) (bFromSweep :type Boolean) (SweepResult :type Hit%20Result%20Structure%20%28by%20ref%29))
  (bind _reftransi (Variables|Default|GetRefTransi))
  (Default|FadeNoir _reftransi)
  (Utilities|FlowControl|Delay 0.75)
  (Utilities|FlowControl|Sequence
    (:then_0
      (switch Utilities|FlowControl|Switch|SwitchonEnumSalle (Variables|Default|GetidTp)
        (:NewEnumerator0
          (Game|LoadStreamLevel(byName) "SalleEntrer1" true)
          (Transformation|SetActorLocation (Variables|Default|GetRefPlayer) (Transformation|GetActorLocation (Variables|Default|GetLieux%20TP)) false true)
          (Utilities|FlowControl|Delay 1.0)
          (Game|UnloadStreamLevel(byName) "SalleApresPortail" false))
        (:NewEnumerator1
          (Game|LoadStreamLevel(byName) "SalleApresPortail" true)
          (Transformation|SetActorLocation (Variables|Default|GetRefPlayer) (Transformation|GetActorLocation (Variables|Default|GetLieux%20TP)) false true)
          (Utilities|FlowControl|Delay 1.0)
          (Game|UnloadStreamLevel(byName) "SalleEntrer1" false)
          (Game|UnloadStreamLevel(byName) "SalleLaby01" false))
        (:NewEnumerator2
          (Game|LoadStreamLevel(byName) "SalleLaby01SaveTest" true)
          (Transformation|SetActorLocation (Variables|Default|GetRefPlayer) (Transformation|GetActorLocation (Variables|Default|GetLieux%20TP)) false true)
          (Utilities|FlowControl|Delay 1.0)
          (Game|UnloadStreamLevel(byName) "SalleApresPortail" false)
          (Game|UnloadStreamLevel(byName) "SalleLaby02" false))
        (:NewEnumerator3
          (Game|LoadStreamLevel(byName) "SalleLaby02" true)
          (Transformation|SetActorLocation (Variables|Default|GetRefPlayer) (Transformation|GetActorLocation (Variables|Default|GetLieux%20TP)) false true)
          (Utilities|FlowControl|Delay 1.0)
          (Game|UnloadStreamLevel(byName) "Sallefin" false)
          (Game|UnloadStreamLevel(byName) "SalleLaby01" false))
        (:NewEnumerator4
          (Game|LoadStreamLevel(byName) "Sallefin" true)
          (Transformation|SetActorLocation (Variables|Default|GetRefPlayer) (Transformation|GetActorLocation (Variables|Default|GetLieux%20TP)) false true)
          (Utilities|FlowControl|Delay 1.0)
          (Game|UnloadStreamLevel(byName) "SalleLaby02" false))))
    (:then_1
      (Default|FadeEnd _reftransi))))

(event EventBeginPlay
  ;[1 1 1] Set le widget de transi
  (bind _returnvalue (UserInterface|CreateWidget "/Game/BluePrintDoss/SpawnPoint/WG_TransiTP.WG_TransiTP_C"))
  (bind _output_get (Variables|Default|SetRefTransi _returnvalue))
  (UserInterface|Viewport|AddtoViewport _output_get 0)
  (bind _asbp_first_person_character (Utilities|Casting|CastToBP_FirstPersonCharacter (Game|GetPlayerCharacter 0)))
  (Variables|Default|SetRefPlayer _asbp_first_person_character))

(fn ConstructionScript)
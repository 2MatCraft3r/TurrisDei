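; NPC shown as a Paper2D flipbook that displays dialogue when the first-person player comes close.
; On BeginPlay it applies the QuelleNPC flipbook and creates a hidden WG_Dialogue widget.
; Tick billboards the sprite toward the player camera on yaw, keeping pitch at zero.
; Player overlap with TriggerDialogue shows the widget and starts QuelleDialoque through Lancement; any end overlap hides it.
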(event OnComponentBeginOverlap(TriggerDialogue)
  (params (OverlappedComponent :type Primitive%20Component%20Object%20Reference) (OtherActor :type Actor%20Object%20Reference) (OtherComp :type Primitive%20Component%20Object%20Reference) (OtherBodyIndex :type Integer) (bFromSweep :type Boolean) (SweepResult :type Hit%20Result%20Structure%20%28by%20ref%29))
  ;[1 1 1] ActiveDialogue
  (Utilities|Casting|CastToBP_FirstPersonCharacter OtherActor)
  (Widget|SetVisibility (Variables|Default|GetRefWidget) "Visible")
  (Default|Lancement (Variables|Default|GetRefWidget) (Variables|Default|GetQuelleDialoque)))

(event OnComponentEndOverlap(TriggerDialogue)
  (params (OverlappedComponent :type Primitive%20Component%20Object%20Reference) (OtherActor :type Actor%20Object%20Reference) (OtherComp :type Primitive%20Component%20Object%20Reference) (OtherBodyIndex :type Integer))
  ;[1 1 1] ActiveDialogue
  (Widget|SetVisibility (Variables|Default|GetRefWidget) "Hidden"))

(event EventBeginPlay
  (Variables|Default|SetSavePoSInitial (Transformation|GetWorldLocation (Variables|Default|GetPaperFlipbook)))
  (bind _returnvalue (UserInterface|CreateWidget "/Game/Widget/Dialogue/WG_Dialogue.WG_Dialogue_C"))
  (bind _output_get (Variables|Default|SetRefWidget _returnvalue))
  (UserInterface|Viewport|AddtoViewport _output_get 0)
  (Widget|SetVisibility _output_get "Hidden")
  (Sprite|SetFlipbook (Variables|Default|GetPaperFlipbook) (Variables|Default|GetQuelleNPC)))

(event EventTick
  (params (DeltaSeconds :type Float%20%28single-precision%29))
  (bind _returnvalue (Game|GetPlayerCharacter 0))
  (bind _paperflipbook (Variables|Default|GetPaperFlipbook))
  (bind _returnvalue_2 (Transformation|GetWorldLocation _paperflipbook))
  (bind _asbp_first_person_character (Utilities|Casting|CastToBP_FirstPersonCharacter _returnvalue))
  (bind _firstpersoncamera (Variables|/Game/FirstPerson/Blueprints/BP_FirstPersonCharacter.BP_FirstPersonCharacter_C|GetFirstPersonCamera _asbp_first_person_character))
  (bind _returnvalue_3 (Transformation|GetWorldLocation _firstpersoncamera))
  (bind _returnvalue_4 (Math|Rotator|FindLookatRotation _returnvalue_2 _returnvalue_3))
  (Transformation|SetWorldRotation (Variables|Default|GetPaperFlipbook) (Math|Rotator|MakeRotator (+ (.roll _returnvalue_4) 0.0) 0.0 (+ (.yaw _returnvalue_4) -9e+01)) false false))

(fn ConstructionScript)